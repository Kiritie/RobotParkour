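; Child tile Blueprint that randomizes a three-lane track segment's layout and coin placement.
; Its construction script calls the parent, picks lane classes, applies them, then flags one random lane and calls coin placement.
; Weighted rolls make all lanes floor half the time, otherwise usually one or occasionally two lanes become empty, blocker or wall.
; At least one lane is always floor, though coin lane selection ignores the layout.
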(event EventBeginPlay)

(event Collision|EventActorBeginOverlap
  (params (OtherActor :type Actor%20Object%20Reference)))

(event EventTick
  (params (DeltaSeconds :type Float%20%28single-precision%29)))

(fn ConstructionScript
  (|CallParentFunction)
  (Utilities|FlowControl|Sequence
    (:then_0
      (|RandomLanes))
    (:then_1
      (CallFunction|SetAllTileComponentClass))
    (:then_2
      (Utilities|Array|SetArrayElem (Variables|Default|GetIsHadPlacedCoins) (Math|Random|RandomInteger 3) true)
      (CallFunction|PlaceAllCoin))))

(fn RandomTileComponentClass
  (switch int (Math|Random|RandomInteger 3)
    (:0
      (LocalVariables|SetTemp 0))
    (:1
      (LocalVariables|SetTemp "/Game/Blueprints/BP_TileComponent_Child_Blocker.BP_TileComponent_Child_Blocker_C"))
    (:2
      (LocalVariables|SetTemp "/Game/Blueprints/BP_TileComponent_Child_Wall.BP_TileComponent_Child_Wall_C")))
  (return (LocalVariables|GetTemp)))