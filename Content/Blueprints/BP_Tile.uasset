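; BP_Tile is a track segment with left, center and right child-actor tile components, apparently for an endless runner.
; When BP_MyCharacter overlaps its Box, it asks BP_MyGameMode to add a random child tile, then destroys itself two seconds later unless the character is dead.
; Helper functions assign each component's class, place coins on flagged components and expose NextTilePos's transform for chaining the following tile.
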(event OnComponentBeginOverlap(Box)
  (params (OverlappedComponent :type Primitive%20Component%20Object%20Reference) (OtherActor :type Actor%20Object%20Reference) (OtherComp :type Primitive%20Component%20Object%20Reference) (OtherBodyIndex :type Integer) (bFromSweep :type Boolean) (SweepResult :type Hit%20Result%20Structure%20%28by%20ref%29))
  (bind _asbp_my_character (Utilities|Casting|CastToBP_MyCharacter OtherActor))
  (bind _asbp_my_game_mode (Utilities|Casting|CastToBP_MyGameMode (Game|GetGameMode)))
  (Default|AddTile _asbp_my_game_mode "/Game/Blueprints/BP_Tile_Child_Random.BP_Tile_Child_Random_C")
  (Utilities|FlowControl|Delay 2.0)
  (if (not (Variables|/Game/Blueprints/Character/BP_MyCharacter.BP_MyCharacter_C|GetIsDead _asbp_my_character))
    (Actor|DestroyActor)))

(event EventBeginPlay)

(event Collision|EventActorBeginOverlap
  (params (OtherActor :type Actor%20Object%20Reference)))

(event EventTick
  (params (DeltaSeconds :type Float%20%28single-precision%29)))

(fn ConstructionScript
  (CallFunction|GetTileComponents))

(fn GetTileComponents
  (bind _tilecomponents (Variables|Default|GetTileComponents))
  (Utilities|Array|SetArrayElem _tilecomponents 0 (Variables|Default|GetLeftTileComponent))
  (Utilities|Array|SetArrayElem _tilecomponents 1 (Variables|Default|GetCenterTileComponent))
  (Utilities|Array|SetArrayElem _tilecomponents 2 (Variables|Default|GetRightTileComponent)))

(fn SetAllTileComponentClass
  (for _index (range 0 2)
    (ChildActorComponent|SetChildActorClass (Utilities|Array|Get(acopy) (Variables|Default|GetTileComponents) _index) (Utilities|Array|Get(acopy) (Variables|Default|GetTileComponentClasses) _index))))

(fn GetNextTileTransform
  (return (Transformation|GetWorldTransform (Variables|Default|GetNextTilePos))))

(fn PlaceAllCoin
  (for _index (range 0 2)
    (if (Utilities|Array|Get(acopy) (Variables|Default|GetIsHadPlacedCoins) _index)
      (bind _asbp_tile_component (Utilities|Casting|CastToBP_TileComponent (Variables|/Script/Engine.ChildActorComponent|GetChildActor (Utilities|Array|Get(acopy) (Variables|Default|GetTileComponents) _index))))
      (Default|PlaceCoin _asbp_tile_component))))