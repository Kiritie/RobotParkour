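; Game mode for an endless-runner style parkour game that builds the starting track and tracks collected coins.
; On BeginPlay it shows the ParkourUI widget, then spawns a run of flat tiles followed by random tiles.
; AddTile chains pieces by spawning each at the stored transform and taking the next one from the new tile.
; IncrementCoin adds a given value to the coin count.
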(event Custom|AddTile
  (params (In :type BP%20Tile%20Class%20Reference))
  ;[1 1 1] 生成地板
  (bind _returnvalue (Game|SpawnActorfromClass In (Variables|Default|GetNextTileTransform) "Undefined" 0 0))
  (bind _out (Default|GetNextTileTransform _returnvalue))
  (Variables|Default|SetNextTileTransform _out))

(event Custom|IncrementCoin
  (params (Value :type Integer))
  ;[1 1 1] 增加金币
  (Variables|Default|SetCoinCount (+ Value (Variables|Default|GetCoinCount))))

(event EventBeginPlay
  (Utilities|FlowControl|Sequence
    (:then_0
      (bind _returnvalue (UserInterface|CreateWidget "/Game/Blueprints/ParkourUI.ParkourUI_C"))
      (UserInterface|Viewport|AddtoViewport _returnvalue 0))
    (:then_1
      (for _index (range 1 5)
        (CallFunction|AddTile "/Game/Blueprints/BP_Tile_Child_Flat.BP_Tile_Child_Flat_C")))
    (:then_2
      (for _index_2 (range 1 15)
        (CallFunction|AddTile "/Game/Blueprints/BP_Tile_Child_Random.BP_Tile_Child_Random_C")))))

(fn ConstructionScript)