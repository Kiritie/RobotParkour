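; Player character for a three-lane runner that moves forward automatically, jumps, and switches lanes.
; Left/right presses fill a two-slot buffer, consumed one at a time by a timeline that lerps Y between lanes and reverses on blocked sweeps or side hits.
; Hit normals on "Blocker"-tagged components distinguish side bumps from fatal head-on crashes.
; Crashes ragdoll the mesh and restart the level after a delay; falling below a height threshold restarts it immediately.
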(event OnComponentHit(CapsuleComponent)
  (params (HitComponent :type Primitive%20Component%20Object%20Reference) (OtherActor :type Actor%20Object%20Reference) (OtherComp :type Primitive%20Component%20Object%20Reference) (NormalImpulse :type Vector :default "0, 0, 0") (Hit :type Hit%20Result%20Structure%20%28by%20ref%29))
  (bind _returnvalue (Transformation|GetActorForwardVector))
  (bind _returnvalue_2 (Math|Vector|DotProduct _returnvalue (.normal Hit)))
  (bind _returnvalue_3 (Math|Float|NearlyEqual(Float) _returnvalue_2 -1.0 0.07))
  ;[1 1 1] 碰撞检测
  (if (Utilities|Name|Equal(Name) (Utilities|Array|Get(acopy) (Variables|/Script/Engine.ActorComponent|GetComponentTags OtherComp)) "Blocker")
    (bind _output_get (Variables|Default|SetIsDead _returnvalue_3))
    (Utilities|FlowControl|Sequence
      (:then_0
        (if (not (or _returnvalue_3 (Math|Float|NearlyEqual(Float) (Math|Vector|DotProduct (Transformation|GetActorUpVector) (.normal Hit)) 1.0 0.07)))
          (Variables|Default|SetIsHitBlockerSide true)))
      (:then_1
        (if _output_get
          (CallFunction|HittoDeath))))))

(event Custom|HandleNewLane
  ;[1 1 1] 处理新道
  (if (and (not (Variables|Default|GetIsChangeLane)) (> (Utilities|Array|Length (Variables|Default|GetKeyBuffer)) 0))
    (bind _output_get (Variables|Default|SetNewLane (+ (Variables|Default|GetCurrentLane) (Utilities|Array|Get(acopy) (Variables|Default|GetKeyBuffer)))))
    (Utilities|Array|RemoveIndex (Variables|Default|GetKeyBuffer))
    (bind _output_get_2 (Variables|Default|SetIsChangeLane (and (>= _output_get 0) (<= _output_get 2))))
    (if _output_get_2
      (CallFunction|StartChangeLane))))

(event Custom|HitToDeath
  (bind _mesh (Variables|Character|GetMesh))
  ;[1 1 1] 撞死
  (Physics|SetSimulatePhysics _mesh true)
  (Collision|SetCollisionEnabled _mesh "QueryAndPhysics")
  (Components|Activation|SetActive (Variables|Character|GetCharacterMovement) false false)
  (Utilities|FlowControl|Delay 2.0)
  (Development|ExecuteConsoleCommand "RestartLevel"))

(event Custom|StartChangeLane
  (bind _returnvalue (Transformation|GetActorLocation))
  (bind _lanes (Variables|Default|GetLanes))
  ;[1 1 1] 执行变道
  (bind (_direction _alpha) (Timeline|ChangeLaneTimeline PlayFromStart)
    (:Update
      (bind _returnvalue_2 (Transformation|SetActorLocation (Math|Vector|MakeVector (.x _returnvalue) (Math|Float|Lerp (Utilities|Array|Get(acopy) _lanes (Variables|Default|GetCurrentLane)) (Utilities|Array|Get(acopy) _lanes (Variables|Default|GetNewLane)) _alpha) (.z _returnvalue)) true false))
      (if (or (not _returnvalue_2) (Variables|Default|GetIsHitBlockerSide))
        (Variables|Default|SetIsHitBlockerSide false)
        (Timeline|ChangeLaneTimeline Reverse)))
    (:Finished
      (Variables|Default|SetIsChangeLane false)
      (switch Utilities|FlowControl|Switch|SwitchonETimelineDirection _direction
        (:Forward
          (Variables|Default|SetCurrentLane (Variables|Default|GetNewLane)))))))

(event Custom|CheckFallToDeath
  ;[1 1 1] 检测摔死
  (if (and (AI|Components|NavMovement|IsFalling (Variables|Character|GetCharacterMovement)) (< (.z (Transformation|GetActorLocation)) -5e+02))
    (Development|ExecuteConsoleCommand "RestartLevel")))

(event EventTick
  (params (DeltaSeconds :type Float%20%28single-precision%29))
  ;[1 1 1] Update
  (if (not (Variables|Default|GetIsDead))
    (CallFunction|CheckFalltoDeath)
    (CallFunction|HandleNewLane)
    (Pawn|Input|AddMovementInput (Math|Vector|GetForwardVector (Pawn|GetControlRotation :!class /Script/Engine.Pawn)) 1.0 false)))

(event Input|ActionEvents|InputActionJump
  (params (Key :type Key%20Structure :default "AnyKey"))
  ;[1 1 1] 跳跃
  (:Pressed
    (if (not (Variables|Default|GetIsDead))
      (Character|Jump)))
  (:Released
    (Character|StopJumping)))

(event Input|ActionEvents|InputActionMoveLeft
  (params (Key :type Key%20Structure :default "AnyKey"))
  ;[1 1 1] 添加按键缓冲
  (:Pressed
    (Variables|Default|SetNewKey -1)
    (if (< (Utilities|Array|Length (Variables|Default|GetKeyBuffer)) 2)
      (Utilities|Array|Add (Variables|Default|GetKeyBuffer) (Variables|Default|GetNewKey)))))

(event Input|ActionEvents|InputActionMoveRight
  (params (Key :type Key%20Structure :default "AnyKey"))
  ;[1 1 1] 添加按键缓冲
  (:Pressed
    (Variables|Default|SetNewKey 1)
    (if (< (Utilities|Array|Length (Variables|Default|GetKeyBuffer)) 2)
      (Utilities|Array|Add (Variables|Default|GetKeyBuffer) (Variables|Default|GetNewKey)))))

(fn ConstructionScript)